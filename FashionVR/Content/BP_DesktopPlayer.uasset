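; BP_DesktopPlayer is a desktop-controlled player character with movement, look, jump and object grabbing.
; On BeginPlay it adds the IMC_Desktop mapping context, and Enhanced Input actions drive camera look, jumping and movement relative to control yaw.
; The E key calls TryGrab on a BPGrabComponent with DesktopGrabController and releases on key up, with debug prints on press.
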(event `EnhancedInput|/Game/XRFramework/Input/Actions/IA_Look`
  (params (ActionValue :type "Vector2D Structure") (ElapsedSeconds :type "Float (double-precision)") (TriggeredSeconds :type "Float (double-precision)") (InputAction :type "InputAction Object Reference" :default "/Game/XRFramework/Input/Actions/IA_Look.IA_Look"))
  (bind (_x _y) (`KismetMathLibrary.BreakVector2D` ActionValue))
  (:`Triggered`
    (`self.AddControllerYawInput` _x)
    (`self.AddControllerPitchInput` _y)))

(event `self.ReceiveBeginPlay`
  (`EnhancedInputSubsystemInterface.AddMappingContext` (pcsubsystem `EnhancedInputLocalPlayerSubsystem` (`GameplayStatics.GetPlayerController` 0)) "/Game/IMC_Desktop.IMC_Desktop" 0 (struct)))

(event `EnhancedInput|/Game/XRFramework/Input/Actions/IA_Move`
  (params (ActionValue :type "Vector2D Structure") (ElapsedSeconds :type "Float (double-precision)") (TriggeredSeconds :type "Float (double-precision)") (InputAction :type "InputAction Object Reference" :default "/Game/XRFramework/Input/Actions/IA_Move.IA_Move"))
  (bind (_x _y) (`KismetMathLibrary.BreakVector2D` ActionValue))
  (bind _returnvalue (`KismetMathLibrary.MakeRotator` 0.0 0.0 (.yaw (`self.GetControlRotation`))))
  (:`Triggered`
    (`self.AddMovementInput` (`KismetMathLibrary.GetForwardVector` _returnvalue) _x)
    (`self.AddMovementInput` (`KismetMathLibrary.GetRightVector` _returnvalue) _y)))

(event `EnhancedInput|/Game/XRFramework/Input/Actions/IA_Jump`
  (params (ActionValue :type Boolean) (ElapsedSeconds :type "Float (double-precision)") (TriggeredSeconds :type "Float (double-precision)") (InputAction :type "InputAction Object Reference" :default "/Game/XRFramework/Input/Actions/IA_Jump.IA_Jump"))
  (:`Started`
    (`self.Jump`))
  (:`Completed`
    (`self.StopJumping`)))

(event `Key|E`
  (params (Key :type "Key Structure"))
  (:`Pressed`
    (`KismetSystemLibrary.PrintString` "E PRESSED")
    (`KismetSystemLibrary.PrintString` "TRY GRAB CALLED")
    (`/Game/XRFramework/Blueprints/BP_GrabComponent.TryGrab` (`self.BP_GrabComponent`) (`self.DesktopGrabController`)))
  (:`Released`
    (`/Game/XRFramework/Blueprints/BP_GrabComponent.TryRelease` (`self.BP_GrabComponent`))))

(fn `UserConstructionScript`)